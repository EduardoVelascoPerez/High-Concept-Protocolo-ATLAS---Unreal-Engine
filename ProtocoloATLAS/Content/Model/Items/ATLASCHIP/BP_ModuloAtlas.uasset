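; BP_ModuloAtlas is an ATLAS module pickup that opens the ATLAS console when the player interacts with it.
; Overlapping its Box with BP_FirstPersonCharacter enables input on the actor and shows the WBP_AvisoE prompt; leaving reverses both.
; Pressing E clears all widgets, adds WBP_AtlasConsole to the viewport at a raised Z-order and destroys the actor, making it single-use.
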(event `self.Box.OnComponentBeginOverlap`
  (params (OverlappedComponent :type "PrimitiveComponent Object Reference") (OtherActor :type "Actor Object Reference") (OtherComp :type "PrimitiveComponent Object Reference") (OtherBodyIndex :type Integer) (bFromSweep :type Boolean) (SweepResult :type "HitResult Structure (by ref)"))
  ; COLISION BOX
  (cast `/Game/FirstPerson/Blueprints/BP_FirstPersonCharacter` OtherActor)
  (`self.EnableInput` (`GameplayStatics.GetPlayerController` 0))
  (bind _returnvalue (`|CreateWidget` "/Game/Widget/WBP_AvisoE.WBP_AvisoE_C"))
  (set `self.Ref_AvisoE` _returnvalue)
  (`UserWidget.AddToViewport` (`self.Ref_AvisoE`) 0))

(event `self.Box.OnComponentEndOverlap`
  (params (OverlappedComponent :type "PrimitiveComponent Object Reference") (OtherActor :type "Actor Object Reference") (OtherComp :type "PrimitiveComponent Object Reference") (OtherBodyIndex :type Integer))
  ; COLISION BOX
  (cast `/Game/FirstPerson/Blueprints/BP_FirstPersonCharacter` OtherActor)
  (`self.DisableInput` (`GameplayStatics.GetPlayerController` 0))
  (`Widget.RemoveFromParent` (`self.Ref_AvisoE`)))

(event `Key|E`
  (params (Key :type "Key Structure"))
  ; Interaccion con ATLAS
  (:`Pressed`
    (set `self.Ref_AvisoE` null)
    (`WidgetLayoutLibrary.RemoveAllWidgets`)
    (`Widget.RemoveFromParent` (`self.Ref_AvisoE`))
    (bind _returnvalue (`|CreateWidget` "/Game/Widget/WBP_AtlasConsole.WBP_AtlasConsole_C"))
    (`UserWidget.AddToViewport` _returnvalue 50)
    (`self.K2_DestroyActor`)))

(fn `UserConstructionScript`)